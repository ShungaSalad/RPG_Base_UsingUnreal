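; BP_StatusEffect_Poison is a status effect Blueprint that periodically changes the health of the actor that owns it.
; On each PeriodicEvent, it finds the owner's BPC_Attributes component and, if valid, applies ValueChange to the Attribute.Main.Health tag.
; The change's origin pairs the owner with the instigator controller.
; BeginPlay and construction add no logic of their own.
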(event `self.PeriodicEvent`
  (bind _returnvalue (`self.GetOwner`))
  (bind _returnvalue_2 (`self.GetComponentByClass` _returnvalue "/Game/RPG_Gacha/Attributes/BPC_Attributes.BPC_Attributes_C"))
  (`/Engine/EditorBlueprintResources/StandardMacros.IsValid` _returnvalue_2
    (:`Is Valid`
      (`/Game/RPG_Gacha/Attributes/BPC_Attributes.ChangeAttribute` _returnvalue_2 (struct :`TagName` "Attribute.Main.Health") "NewEnumerator3" (`self.Value Change`) (make `/Game/RPG_Gacha/S_Origin` _returnvalue (`self.GetInstigatorController`))))))

(fn `UserConstructionScript`
  (`parent.UserConstructionScript`))