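; Ability manager component that gives its owning Pawn a set of usable abilities in the RPG.
; It caches the owner on BeginPlay, then spawns each ability class as an actor with that Pawn as Owner and Instigator.
; Each spawned actor joins the available list, and a change notification fires with the updated list after every addition.
; Abilities are used by list index, with the actual attempt delegated to the ability actor.
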(event `self.ReceiveBeginPlay`
  (bind _aspawn (cast `Pawn` (`self.GetOwner`)))
  (set `self.OwnerRef` _aspawn))

(fn `AddAbilityByClass`
  (params (AbilityClass :type "/Game/RPG_Gacha/Abilities/BP_Ability Class Reference"))
  (bind _ownerref (`self.OwnerRef`))
  (bind _returnvalue (`|SpawnActorFromClass` AbilityClass (`KismetMathLibrary.MakeTransform` (0.0 0.0 0.0)) "Undefined" "MultiplyWithRoot" _ownerref _ownerref))
  (`KismetArrayLibrary.Array_Add` (`self.AvailableAbilities`) _returnvalue)
  (`self.AbilitiesAvailableChanged` (`self.AvailableAbilities`))
  (return))

(fn `InitializeAbilities`
  (params (KnownAbilities :type "Array of /Game/RPG_Gacha/Abilities/BP_Ability Class Reference"))
  (for _array_element KnownAbilities
    (`self.AddAbilityByClass` _array_element))
  (return))

(fn `UseAbility`
  (params (AbilityIndex :type Integer))
  (`/Game/RPG_Gacha/Abilities/BP_Ability.AttemptUseAbility` (`|GetArrayItem` (`self.AvailableAbilities`) AbilityIndex))
  (return))