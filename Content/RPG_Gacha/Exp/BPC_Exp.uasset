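; BPC_Exp is an actor component that handles experience and leveling, and grants experience to whoever kills its owner.
; It listens for the State.Dead gameplay tag and passes ExpToAward to the BPC_Exp on the origin controller's pawn.
; AwardExp adds to a running total, then recursively levels up against LevelCurve thresholds until MaxLevel.
; It broadcasts LevelUp and ExpChanged events, though ExpChanged always reports level 0.
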(event `self.ReceiveBeginPlay`
  (`/Game/RPG_Gacha/GameplayTags/BPC_GameplayTags.AddTagListener` (`Actor.GetComponentByClass` (`self.GetOwner`) "/Game/RPG_Gacha/GameplayTags/BPC_GameplayTags.BPC_GameplayTags_C") (struct :`TagName` "State.Dead") (delegate `DeadStateUpdate`)))

(event `DeadStateUpdate`
  (params (GameplayTagContext :type "/Game/RPG_Gacha/GameplayTags/S_GameplayContext Structure"))
  (bind (_contexttag _activetags _origin) (break `/Game/RPG_Gacha/GameplayTags/S_GameplayContext` GameplayTagContext))
  (bind (_actor _controller) (break `/Game/RPG_Gacha/S_Origin` _origin))
  (bind _returnvalue (`Controller.K2_GetPawn` _controller))
  (bind _returnvalue_2 (`Actor.GetComponentByClass` _returnvalue "BPC_Exp_C"))
  (if (`BlueprintGameplayTagLibrary.HasTag` _activetags (struct :`TagName` "State.Dead"))
    (`/Engine/EditorBlueprintResources/StandardMacros.IsValid` _controller
      (:`Is Valid`
        (`/Engine/EditorBlueprintResources/StandardMacros.IsValid` _returnvalue
          (:`Is Valid`
            (`/Engine/EditorBlueprintResources/StandardMacros.IsValid` _returnvalue_2
              (:`Is Valid`
                (`self.AwardExp` _returnvalue_2 (`self.ExpToAward`))))))))))

(event `AwardExp`
  (params (AwardedExp :type "Float (double-precision)"))
  (bind _output_get (set `self.CurrentExp` (+ AwardedExp (`self.CurrentExp`))))
  (`self.TryToLevelUp`)
  (`self.ExpChanged` (make `/Game/RPG_Gacha/Exp/S_ExpContext` _output_get)))

(event `Signature` :!signature `self.ExpChanged`
  (params (ExpContext :type "/Game/RPG_Gacha/Exp/S_ExpContext Structure")))

(fn `LevelUpCondition`
  (returns (LeveledUp :type Boolean))
  (if (== (`self.CurrentLevel`) (`self.MaxLevel`))
    (return false)
    (elif (>= (`self.CurrentExp`) (`CurveFloat.GetFloatValue` (`self.LevelCurve`) (`KismetMathLibrary.Conv_IntToDouble` (+ (`self.CurrentLevel`) 1))))
      (`/Engine/EditorBlueprintResources/StandardMacros.IncrementInt` (`self.CurrentLevel`)
        (:`  `
          (return true)))
      (else
        (return false)))))

(fn `TryToLevelUp`
  (bind _leveledup (`self.LevelUpCondition`))
  (if _leveledup
    (`self.LevelUp` (make `/Game/RPG_Gacha/Exp/S_ExpContext` (`self.CurrentExp`) (`self.CurrentLevel`)))
    (`KismetSystemLibrary.PrintString` "Leveled Up")
    (`self.TryToLevelUp`)
    (return)
    (else
      (return))))