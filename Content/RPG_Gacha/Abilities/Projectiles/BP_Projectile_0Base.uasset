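; Base projectile actor for RPG abilities that damages what it overlaps or hits, then destroys itself.
; Construction sets movement speeds from ProjectileStats, and overlaps skip the owner and actors tagged State.Dead.
; Destruction rolls a critical from the owner's attribute component, applying that damage to pawns within the optional explosion radius.
; Single-target hits apply unmodified base damage, and the looping IncreaseVelocity timer event is empty.
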(event `self.ReceiveBeginPlay`
  (`KismetSystemLibrary.K2_SetTimerDelegate` (delegate `IncreaseVelocity`) 1.0 true))

(event `IncreaseVelocity`)

(event `self.Sphere.OnComponentBeginOverlap`
  (params (OverlappedComponent :type "PrimitiveComponent Object Reference") (OtherActor :type "Actor Object Reference") (OtherComp :type "PrimitiveComponent Object Reference") (OtherBodyIndex :type Integer) (bFromSweep :type Boolean) (SweepResult :type "HitResult Structure (by ref)"))
  (if (!= OtherActor (`self.GetOwner`))
    (if (`.ReturnValue` (`BlueprintMapLibrary.Map_Find` (`/Game/RPG_Gacha/GameplayTags/BPC_GameplayTags.StackedTags` (`self.GetComponentByClass` OtherActor "/Game/RPG_Gacha/GameplayTags/BPC_GameplayTags.BPC_GameplayTags_C")) "State.Dead"))
      (`KismetSystemLibrary.PrintString` "DEAD!!!!")
      (else
        (`KismetSystemLibrary.PrintString` "Overlapped")
        (`self.Destruction` OtherActor)))))

(event `self.ReceiveHit`
  (params (MyComp :type "PrimitiveComponent Object Reference") (Other :type "Actor Object Reference") (OtherComp :type "PrimitiveComponent Object Reference") (bSelfMoved :type Boolean) (HitLocation :type "Vector Structure") (HitNormal :type "Vector Structure") (NormalImpulse :type "Vector Structure") (Hit :type "HitResult Structure (by ref)"))
  (`KismetSystemLibrary.PrintString` "Hit")
  (`self.Destruction` Other))

(event `Destruction`
  (params (HitActor :type "Actor Object Reference"))
  (bind _attributefound (`/Game/RPG_Gacha/Attributes/BPC_Attributes.GetAttributeFromTag` (`self.GetComponentByClass` (`self.GetOwner`) "/Game/RPG_Gacha/Attributes/BPC_Attributes.BPC_Attributes_C") (struct :`TagName` "Attribute.Main.Crit_Rate")))
  (bind _critical (`/Game/RPG_Gacha/FunctionLibrary/BPFL_CriticalCheck.IsCritical` _attributefound))
  (bind _attributefound_2 (`/Game/RPG_Gacha/Attributes/BPC_Attributes.GetAttributeFromTag` (`self.GetComponentByClass` (`self.GetOwner`) "/Game/RPG_Gacha/Attributes/BPC_Attributes.BPC_Attributes_C") (struct :`TagName` "Attribute.Main.Crit_Dmg")))
  (bind _finaldamage (`/Game/RPG_Gacha/FunctionLibrary/BPFL_CriticalDamageCalculation.CalculateCriticalDamageValue` _attributefound_2 _critical (`.Damage_3_39976B094F6E4BA6C059E79F947FF40B` (break `/Game/RPG_Gacha/Abilities/Projectiles/S_ProjectileStats` (`self.ProjectileStats`)))))
  (set `self.FinalDamage` _finaldamage)
  (if (`.HasExplosionRadius_9_5865F64F486B397A18FA238B85FD94EC` (break `/Game/RPG_Gacha/Abilities/Projectiles/S_ProjectileStats` (`self.ProjectileStats`)))
    (if (`self.DrawDebug`)
      (`KismetSystemLibrary.DrawDebugSphere` (`self.K2_GetActorLocation`) (`.ExplosionRadius_6_C8EF06ED40A100ACF355CDB81B225B54` (break `/Game/RPG_Gacha/Abilities/Projectiles/S_ProjectileStats` (`self.ProjectileStats`))) 12 (struct :`R` 1.0 :`G` 1.0 :`B` 1.0 :`A` 1.0) 5.0 1.0))
    (bind _outactors (`KismetSystemLibrary.SphereOverlapActors` (`self.K2_GetActorLocation`) (`.ExplosionRadius_6_C8EF06ED40A100ACF355CDB81B225B54` (break `/Game/RPG_Gacha/Abilities/Projectiles/S_ProjectileStats` (`self.ProjectileStats`))) (`|MakeArray` "ObjectTypeQuery3" :!type "EObjectTypeQuery Enum") null (`|MakeArray` (`self.GetOwner`) null)))
    (for _array_element _outactors
      (`GameplayStatics.ApplyDamage` _array_element (`self.FinalDamage`) (`self.GetInstigatorController`) self))
    (else
      (`GameplayStatics.ApplyDamage` HitActor (`.Damage_3_39976B094F6E4BA6C059E79F947FF40B` (break `/Game/RPG_Gacha/Abilities/Projectiles/S_ProjectileStats` (`self.ProjectileStats`))) (`self.GetInstigatorController`) self)))
  (`self.K2_DestroyActor`))

(fn `UserConstructionScript`
  (bind _projectilemovement (`self.ProjectileMovement`))
  (bind ((`Speed_4_B757057845BCFC0439D6BEA990C7A63E` _speed) (`MaxSpeed_12_21C96FFE4671F67D883262AB584A2119` _maxspeed)) (break `/Game/RPG_Gacha/Abilities/Projectiles/S_ProjectileStats` (`self.ProjectileStats`)))
  (set `ProjectileMovementComponent.InitialSpeed` _speed _projectilemovement)
  (set `ProjectileMovementComponent.MaxSpeed` _maxspeed _projectilemovement))