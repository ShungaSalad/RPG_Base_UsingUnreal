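; Periodic buff status effect that heals its owner in proportion to missing health.
; On each periodic event it reads Health from the owner's BPC_Attributes and takes Max minus BaseValue as the amount lost.
; It splits ValueModifierPercent across the tick count (Duration / PeriodicTime) and applies that share via ChangeAttribute, crediting the instigator's controller.
; Missing health is re-read every tick rather than captured once.
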(event `self.PeriodicEvent`
  (bind _returnvalue (`self.GetOwner`))
  (bind (_duration _periodictime) (break `/Game/RPG_Gacha/StatusEffects/S_StatusEffect` (`self.StatusEffectInfo`)))
  (bind _returnvalue_2 (`self.GetComponentByClass` _returnvalue "/Game/RPG_Gacha/Attributes/BPC_Attributes.BPC_Attributes_C"))
  (`/Engine/EditorBlueprintResources/StandardMacros.IsValid` _returnvalue_2
    (:`Is Valid`
      (bind _attributefound (`/Game/RPG_Gacha/Attributes/BPC_Attributes.GetAttributeFromTag` _returnvalue_2 (struct :`TagName` "Attribute.Main.Health")))
      (bind (_basevalue _delta _multiplier _max) (break `/Game/RPG_Gacha/Attributes/S_Attribute` _attributefound))
      (set `self.AmountLost` (- _max _basevalue))
      (`/Game/RPG_Gacha/Attributes/BPC_Attributes.ChangeAttribute` _returnvalue_2 (struct :`TagName` "Attribute.Main.Health") "NewEnumerator1" (* (/ (/ (`self.Value Modifier Percent`) (/ _duration _periodictime)) 100.0) (`self.AmountLost`)) (make `/Game/RPG_Gacha/S_Origin` _returnvalue (`self.GetInstigatorController`))))))

(fn `UserConstructionScript`
  (`parent.UserConstructionScript`))