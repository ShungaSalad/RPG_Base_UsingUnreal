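; BP_Ability_Shoot is an ability that fires a projectile from its owner when the animation apex event triggers.
; It reads the owner's Attack attribute from BPC_Attributes, then has BPC_Combat launch the configured projectile class with freshly built stats.
; CreateProjectileStats scales damage linearly by ability level and power multiplier, and passes along speed and optional explosion radius settings.
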(event `self.AnimationApexEvent`
  (bind _attributefound (`/Game/RPG_Gacha/Attributes/BPC_Attributes.GetAttributeFromTag` (`self.GetComponentByClass` (`self.GetOwner`) "/Game/RPG_Gacha/Attributes/BPC_Attributes.BPC_Attributes_C") (struct :`TagName` "Attribute.Main.Attack")))
  (bind _calculatevalue (`/Game/RPG_Gacha/FunctionLibrary/BPFL_AttributeHelper.CalculateAttributeValue` _attributefound))
  (`/Game/RPG_Gacha/Combat/BPC_Combat.FireProjectile` (`self.GetComponentByClass` (`self.GetOwner`) "/Game/RPG_Gacha/Combat/BPC_Combat.BPC_Combat_C") (`self.Projectile`) (`self.CreateProjectileStats` _calculatevalue)))

(fn `CreateProjectileStats`
  (params (Attack :type "Float (double-precision)"))
  (returns (S_ProjectileStats :type "/Game/RPG_Gacha/Abilities/Projectiles/S_ProjectileStats Structure"))
  (return (make `/Game/RPG_Gacha/Abilities/Projectiles/S_ProjectileStats` (* Attack (* (`self.CurrentAbilityLevel`) (`self.PowerMultiplier`))) (`self.InitialProjectileSpeed`) (`self.FinalProjectileSpeed`) (`self.ExplosionRadius`) (`self.HasExplosionRadius`))))

(fn `UserConstructionScript`
  (`parent.UserConstructionScript`))