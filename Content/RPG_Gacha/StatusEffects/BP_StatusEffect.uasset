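; Base timed status effect for the RPG, acting on its owner's gameplay tag, attribute and status effect components.
; AttemptApplication checks required and preventing tags, then starts the effect or requests its removal.
; Starting adds tags, applies level-curve-scaled attribute changes and sets duration and looping periodic timers; PeriodicEvent is an empty hook.
; Ending removes the tags, negates the attribute changes, clears timers and removes itself from BPC_StatusEffects.
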(event `AttemptApplication`
  (bind _applystatuseffect (`self.CheckTagStartConditions`))
  (if _applystatuseffect
    (`self.StartStatusEffect`)
    (else
      (`self.AttemptRemoveStatusEffects`))))

(event `StartStatusEffect`
  (bind (_duration _periodictime) (break `/Game/RPG_Gacha/StatusEffects/S_StatusEffect` (`self.StatusEffectInfo`)))
  (`self.AddTags`)
  (`self.ApplyAttributeEffects` true)
  (bind _returnvalue (`KismetSystemLibrary.K2_SetTimerDelegate` (delegate `PeriodicEvent`) _periodictime true))
  (set `self.PeriodicTimerHandle` _returnvalue)
  (bind _returnvalue_2 (`KismetSystemLibrary.K2_SetTimerDelegate` (delegate `EndStatusEffect`) _duration false 0.001))
  (set `self.DurationTimerHandle` _returnvalue_2))

(event `EndStatusEffect`
  (`self.RemoveTags`)
  (`self.ApplyAttributeEffects` false)
  (`self.ClearTimers`)
  (`self.AttemptRemoveStatusEffects`))

(event `PeriodicEvent`)

(fn `AddTags`
  (bind _returnvalue (`self.GetOwner`))
  (for _array_element (`self.AddingTags`)
    (`/Game/RPG_Gacha/GameplayTags/BPC_GameplayTags.AddTag` (`self.GetComponentByClass` _returnvalue "/Game/RPG_Gacha/GameplayTags/BPC_GameplayTags.BPC_GameplayTags_C") _array_element (make `/Game/RPG_Gacha/S_Origin` _returnvalue (`self.GetInstigatorController` _returnvalue))))
  (return))

(fn `ApplyAttributeEffects`
  (params (AddEffects :type Boolean))
  (locals (LocalMultiplier :type "Float (double-precision)"))
  (bind _returnvalue (`self.GetOwner`))
  (bind _returnvalue_2 (`self.GetComponentByClass` (`self.GetOwner`) "/Game/RPG_Gacha/Attributes/BPC_Attributes.BPC_Attributes_C"))
  (if AddEffects
    (set `local.LocalMultiplier` 1.0)
    (else
      (set `local.LocalMultiplier` -1.0)))
  (`/Engine/EditorBlueprintResources/StandardMacros.IsValid` _returnvalue_2
    (:`Is Valid`
      (for _array_element (`self.AttributeEffects`)
        (bind (_attributetochange _changetype _powermultiplier _scalingcurve) (break `/Game/RPG_Gacha/StatusEffects/S_AttributeChange` _array_element))
        (`/Game/RPG_Gacha/Attributes/BPC_Attributes.ChangeAttribute` _returnvalue_2 _attributetochange _changetype (* (* _powermultiplier (`CurveFloat.GetFloatValue` _scalingcurve (`self.Level`))) (`local.LocalMultiplier`)) (make `/Game/RPG_Gacha/S_Origin` _returnvalue (`self.GetInstigatorController` _returnvalue))))
      (return))
    (:`Is Not Valid`
      (return))))

(fn `CheckTagStartConditions`
  (returns (ApplyStatusEffect :type Boolean))
  (bind _tagcontainer (`/Game/RPG_Gacha/GameplayTags/BPC_GameplayTags.GetActiveTagContainer` (`self.GetComponentByClass` (`self.GetOwner`) "/Game/RPG_Gacha/GameplayTags/BPC_GameplayTags.BPC_GameplayTags_C")))
  (return (and (`BlueprintGameplayTagLibrary.HasAllTags` _tagcontainer (`self.RequiredTags`)) (not (`BlueprintGameplayTagLibrary.HasAnyTags` _tagcontainer (`self.PreventingTags`))))))

(fn `ClearTimers`
  (`KismetSystemLibrary.K2_ClearAndInvalidateTimerHandle` (`self.PeriodicTimerHandle`))
  (`KismetSystemLibrary.K2_ClearAndInvalidateTimerHandle` (`self.DurationTimerHandle`))
  (return))

(fn `RemoveTags`
  (bind _returnvalue (`self.GetOwner`))
  (for _array_element (`self.AddingTags`)
    (`/Game/RPG_Gacha/GameplayTags/BPC_GameplayTags.RemoveTag` (`self.GetComponentByClass` _returnvalue "/Game/RPG_Gacha/GameplayTags/BPC_GameplayTags.BPC_GameplayTags_C") _array_element (make `/Game/RPG_Gacha/S_Origin` _returnvalue (`self.GetInstigatorController` _returnvalue))))
  (return))

(fn `UserConstructionScript`)